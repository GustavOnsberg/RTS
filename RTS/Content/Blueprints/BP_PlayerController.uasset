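; Player controller that places buildings in the world on left mouse click.
; The click traces under the cursor on the Visibility channel, snaps X and Y to a 100-unit grid and keeps the hit Z.
; PlaceBuildingInHand always spawns a hardcoded BP_Building_SmallHouse there, ignoring collision, with no check that the trace hit anything.
; A debug "Hello" prints after each placement.
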(event Custom|PlaceBuildingInHand
  (params (Location :type Vector))
  (Game|SpawnActorfromClass "/Game/Blueprints/Buildings/BP_Building_SmallHouse.BP_Building_SmallHouse_C" (Math|Transform|MakeTransform Location "0, 0, 0" "1,1,1") "AlwaysSpawn" self 0))

(event EventBeginPlay)

(event EventTick
  (params (DeltaSeconds :type Float%20%28single-precision%29)))

(event Input|MouseEvents|LeftMouseButton
  (params (Key :type Key%20Structure :default "AnyKey"))
  (bind _hitresult (Game|Player|GetHitResultUnderCursorbyChannel "TraceTypeQuery1" true))
  (bind (_x _y _z) (Math|Vector|BreakVector (.location _hitresult)))
  (:Pressed
    (CallFunction|PlaceBuildinginHand (Math|Vector|MakeVector (* (Math|Float|Round (/ _x 1e+02)) 1e+02) (* (Math|Float|Round (/ _y 1e+02)) 1e+02) _z))
    (Development|PrintString "Hello")))

(fn ConstructionScript)