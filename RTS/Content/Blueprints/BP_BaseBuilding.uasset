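; Base building actor that validates whether it can be placed at its current location and shows the result by swapping the mesh material.
; The construction script scales a CollisionTester to the Width and Length footprint, and any overlapping actor blocks placement.
; Otherwise, a grid of downward traces across the footprint rejects missing ground or height differing too far from the center.
; OnPlace is an empty function.
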(event EventBeginPlay)

(event Collision|EventActorBeginOverlap
  (params (OtherActor :type Actor%20Object%20Reference)))

(event EventTick
  (params (DeltaSeconds :type Float%20%28single-precision%29)))

(fn ConstructionScript
  (Transformation|SetRelativeScale3D (Variables|Default|GetCollisionTester) (Math|Vector|MakeVector (Math|Conversions|ToFloat(Integer) (Variables|Default|GetWidth)) (Math|Conversions|ToFloat(Integer) (Variables|Default|GetLength)) 0.2)))

(fn OnPlace)

(fn CheckifCanbePlaced
  (bind _returnvalue (Transformation|GetActorLocation))
  (bind _returnvalue_2 (Transformation|GetActorLocation))
  (if (> (Utilities|Array|Length (Collision|GetOverlappingActors (Variables|Default|GetCollisionTester) 0 :!class /Script/Engine.PrimitiveComponent)) 0)
    (Rendering|Material|SetMaterial (Variables|Default|GetBuildingMesh) 0 "/Game/Materials/Mat_CanNotPlace.Mat_CanNotPlace")
    (return false)
    (else
      (bind _outhit (Collision|LineTraceByChannel _returnvalue_2 (- _returnvalue_2 "0, 0,200.000000") "TraceTypeQuery1" false 0 "None"))
      (Variables|Default|SetHouseCenterGroundHeight (- (.z (.tracestart _outhit)) (.z (.location _outhit))))
      (for _index (range 0 (Variables|Default|GetLength))
        (for _index_2 (range 0 (Variables|Default|GetWidth))
          (bind _outhit_2 (Collision|LineTraceByChannel (Math|Vector|MakeVector (+ (.x _returnvalue) (* (- (Math|Conversions|ToFloat(Integer) _index_2) (/ (Math|Conversions|ToFloat(Integer) (Variables|Default|GetWidth)) 2.0)) 1e+02)) (+ (.y _returnvalue) (* (- (Math|Conversions|ToFloat(Integer) _index) (/ (Math|Conversions|ToFloat(Integer) (Variables|Default|GetLength)) 2.0)) 1e+02)) (.z _returnvalue)) (Math|Vector|MakeVector (+ (.x _returnvalue) (* (- (Math|Conversions|ToFloat(Integer) _index_2) (/ (Math|Conversions|ToFloat(Integer) (Variables|Default|GetWidth)) 2.0)) 1e+02)) (+ (.y _returnvalue) (* (- (Math|Conversions|ToFloat(Integer) _index) (/ (Math|Conversions|ToFloat(Integer) (Variables|Default|GetLength)) 2.0)) 1e+02)) (- (.z _returnvalue) 2e+02)) "TraceTypeQuery1" false 0 "None"))
          (if (or (not (.bblockinghit _outhit_2)) (> (Math|Float|Absolute(Float) (- (Variables|Default|GetHouseCenterGroundHeight) (- (.z (.tracestart _outhit_2)) (.z (.location _outhit_2))))) 5e+01))
            (Rendering|Material|SetMaterial (Variables|Default|GetBuildingMesh) 0 "/Game/Materials/Mat_CanNotPlace.Mat_CanNotPlace")
            (return false))))
      (Rendering|Material|SetMaterial (Variables|Default|GetBuildingMesh) 0 "/Game/Materials/Mat_CanPlace.Mat_CanPlace")
      (return true))))