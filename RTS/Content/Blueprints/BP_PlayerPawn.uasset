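; Top-down player pawn for a city-builder style camera with a grid-snapped house placement preview.
; Axis input pans the camera at a speed scaled by its height, and action input steps that height within clamped limits.
; BeginPlay spawns a small house, which the building tick moves to the cursor trace hit, rounded to a 100-unit XY grid.
; Placement is unfinished: PlaceHouseInHand only destroys the held house and is not called here.
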(event EventBeginPlay
  (CallFunction|SpawnHousetoPlace))

(event Collision|EventActorBeginOverlap
  (params (OtherActor :type Actor%20Object%20Reference)))

(event EventTick
  (params (DeltaSeconds :type Float%20%28single-precision%29))
  (Utilities|FlowControl|Sequence
    (:then_0
      (CallFunction|TickBuilding))))

(event Input|ActionEvents|InputActionMoveCameraDown
  (params (Key :type Key%20Structure :default "AnyKey"))
  (bind _returnvalue (Transformation|GetActorLocation))
  (:Pressed
    (Transformation|SetActorLocation (Math|Vector|MakeVector (.x _returnvalue) (.y _returnvalue) (Math|Float|Clamp(Float) (- (.z _returnvalue) 1.5e+02) 5e+02 1e+04)) false false)))

(event Input|ActionEvents|InputActionMoveCameraUp
  (params (Key :type Key%20Structure :default "AnyKey"))
  (bind _returnvalue (Transformation|GetActorLocation))
  (:Pressed
    (Transformation|SetActorLocation (Math|Vector|MakeVector (.x _returnvalue) (.y _returnvalue) (Math|Float|Clamp(Float) (+ (.z _returnvalue) 1.5e+02) 5e+02 1e+04)) false false)))

(event Input|AxisEvents|InputAxisMoveCameraRight
  (params (AxisValue :type Float%20%28single-precision%29))
  (Transformation|AddActorWorldOffset (* (Transformation|GetActorRightVector) (* AxisValue (Variables|Default|GetCameraSpeed) (Utilities|Time|GetWorldDeltaSeconds) (.z (Transformation|GetActorLocation))))))

(event Input|AxisEvents|InputAxisMoveCameraForward
  (params (AxisValue :type Float%20%28single-precision%29))
  (Transformation|AddActorWorldOffset (* (Transformation|GetActorForwardVector) (* AxisValue (Variables|Default|GetCameraSpeed) (Utilities|Time|GetWorldDeltaSeconds) (.z (Transformation|GetActorLocation))))))

(event Custom|Tick_Building
  (Variables|Default|SetLocationUnderCursor (.location (.HitResult (Game|Player|GetHitResultUnderCursorbyChannel (Game|GetPlayerController 0) "TraceTypeQuery1" true))))
  (CallFunction|MoveHouseinHand))

(event Custom|MoveHouseInHand
  (bind _locationundercursor (Variables|Default|GetLocationUnderCursor))
  (bind (_x _y _z) (Math|Vector|BreakVector _locationundercursor))
  (Transformation|SetActorLocation (Variables|Building|GetBuildingToPlace) (Math|Vector|MakeVector (* (Math|Float|Round (/ _x 1e+02)) 1e+02) (* (Math|Float|Round (/ _y 1e+02)) 1e+02) _z) false false))

(event Custom|PlaceHouseInHand
  (Actor|DestroyActor (Variables|Building|GetBuildingToPlace)))

(event Custom|SpawnHouseToPlace
  (bind _returnvalue (Game|SpawnActorfromClass "/Game/Blueprints/Buildings/BP_Building_SmallHouse.BP_Building_SmallHouse_C" (Math|Transform|MakeTransform "0, 0, 0" "0, 0, 0" "1,1,1") "AlwaysSpawn" self 0))
  (Variables|Building|SetBuildingToPlace _returnvalue))

(fn ConstructionScript)

(fn OnRepLocationUnderCursor)