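; Player controller for the main menu that shows the menu UI and starts hosting or joining lobbies.
; On BeginPlay it creates the UI_MainMenu widget and adds it to the viewport.
; CreateLobby and JoinLobby events forward to BP_GameInstance, passing itself and, for hosting, its connection count and LAN settings.
; A failed game instance cast only prints an error.
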(event Custom|CreateLobby
  (bind _asbp_game_instance (Utilities|Casting|CastToBP_GameInstance (Game|GetGameInstance))
    (:then
      (Default|InstanceHostLobby _asbp_game_instance self (Variables|Default|GetHostPublicConnections) (Variables|Default|GetHostLAN)))
    (:CastFailed
      (Development|PrintString "Game instance not found" true true "(R=1.000000,G=0.000000,B=0.000000,A=1.000000)"))))

(event Custom|JoinLobby
  (bind _asbp_game_instance (Utilities|Casting|CastToBP_GameInstance (Game|GetGameInstance))
    (:then
      (Default|InstanceJoinLobby _asbp_game_instance self))
    (:CastFailed
      (Development|PrintString "Game instance not found" true true "(R=1.000000,G=0.000000,B=0.000000,A=1.000000)"))))

(event EventBeginPlay
  (bind _returnvalue (UserInterface|CreateWidget "/Game/UI/UI_MainMenu.UI_MainMenu_C"))
  (UserInterface|Viewport|AddtoViewport _returnvalue 0))

(event EventTick
  (params (DeltaSeconds :type Float%20%28single-precision%29)))

(fn ConstructionScript)